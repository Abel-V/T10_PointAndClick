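; Player controller for point-and-click movement, sending the pawn toward the location under the cursor.
; Each left press traces the cursor and calls MoveToLocation, which runs SimpleMoveToLocation unless the goal is under 100 units away.
; A click counter, reset shortly after release through a retriggerable delay, detects double clicks and raises walk speed to run.
; A Tick-fed Gate tracks the held button for continuous movement, but its exit drives nothing.
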(event `self.ReceiveTick`
  (params (DeltaSeconds :type "Float (single-precision)"))
  ;[1 1 1] T12 - Si dejamos click izq pulsado, el personaje va al destino continuamente
  (`/Engine/EditorBlueprintResources/StandardMacros.Gate` true :!label _label) ; De este modo, cuando pulsamos el ratón se ejecutará el código \nque haya después del semáforo, y cuando lo soltemos se parará el semáforo. \nY este módulo se ejecutará en cada frame, es decir, conectamos Enter \na la salida de un evento Tick.
)

(event `InputAction|LeftClick`
  (params (Key :type "Key Structure"))
  ;[1 1 1] T12 - Si dejamos click izq pulsado, el personaje va al destino continuamente
  (:`Pressed`
    (goto _label :!via `Open`))
  (:`Released`
    (goto _label :!via `Close`)))

(event `InputAction|LeftClick`
  (params (Key :type "Key Structure"))
  (bind _hitresult (`self.GetHitResultUnderCursorByChannel` "TraceTypeQuery1"))
  (bind _charactermovement (`Character.CharacterMovement` (`GameplayStatics.GetPlayerCharacter` 0)))
  ;[1 1 1] T12 ej3 - Hacer que corra si se ha dado doble click en vez de uno
  ;;[1 1 1] Detectar doble click
  (:`Pressed`
    (bind _result (`/Engine/EditorBlueprintResources/StandardMacros.IncrementInt` (`self.Click Count`))
      (:`  `
        (if (>= _result 2)
          (set `CharacterMovementComponent.MaxWalkSpeed` 900.0 _charactermovement)
          (`self.MoveToLocation` _hitresult)
          (else
            (set `CharacterMovementComponent.MaxWalkSpeed` 500.0 _charactermovement)
            (`self.MoveToLocation` _hitresult))))))
  (:`Released`
    (`KismetSystemLibrary.RetriggerableDelay` 0.2)
    (set `self.Click Count` 0)))

(fn `MoveToLocation`
  (params (HitResult :type "HitResult Structure"))
  (bind (_bblockinghit _binitialoverlap _time _distance _location) (`GameplayStatics.BreakHitResult` HitResult))
  (if (>= (`KismetMathLibrary.VSize` (- (`self.K2_GetActorLocation` (`self.K2_GetPawn`)) _location)) 100.0)
    (`AIBlueprintHelperLibrary.SimpleMoveToLocation` self _location)))

(fn `UserConstructionScript`)