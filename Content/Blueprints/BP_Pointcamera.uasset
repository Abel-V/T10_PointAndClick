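; Camera actor that slowly turns Camera1 to track the first player's character while FollowPlayer is set.
; Each Tick interpolates the camera's forward vector toward the player offset, converts it to pitch and yaw, and zeroes roll.
; Angle clamps derive from that same new rotation rather than fixed limits, with pitch's minimum taken from yaw.
; When FollowPlayer is off, Tick only sets a wide field of view.
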(event `self.ReceiveTick`
  (params (DeltaSeconds :type "Float (single-precision)"))
  (bind _pitch (.pitch (`KismetMathLibrary.MakeRotFromX` (`KismetMathLibrary.VInterpTo` (`KismetMathLibrary.Conv_RotatorToVector` (`SceneComponent.K2_GetComponentRotation` (`self.Camera1`))) (- (`self.K2_GetActorLocation` (`GameplayStatics.GetPlayerCharacter` 0)) (`SceneComponent.K2_GetComponentLocation` (`self.Camera1`))) DeltaSeconds 0.1))))
  (bind _yaw (.yaw (`KismetMathLibrary.MakeRotFromX` (`KismetMathLibrary.VInterpTo` (`KismetMathLibrary.Conv_RotatorToVector` (`SceneComponent.K2_GetComponentRotation` (`self.Camera1`))) (- (`self.K2_GetActorLocation` (`GameplayStatics.GetPlayerCharacter` 0)) (`SceneComponent.K2_GetComponentLocation` (`self.Camera1`))) DeltaSeconds 0.1))))
  (if (`self.Follow Player`)
    (`SceneComponent.K2_SetWorldRotation` (`self.Camera1`) (`KismetMathLibrary.MakeRotator` 0.0 (`KismetMathLibrary.ClampAngle` _pitch (- _yaw 80.0) (+ _pitch 80.0)) (`KismetMathLibrary.ClampAngle` _yaw (- _yaw 80.0) (+ _yaw 80.0))) false false)
    (else
      (`CameraComponent.SetFieldOfView` (`self.Camera1`) 120.0))))

(fn `UserConstructionScript`)